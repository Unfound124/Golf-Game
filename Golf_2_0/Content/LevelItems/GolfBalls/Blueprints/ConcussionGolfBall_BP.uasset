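; Concussion golf ball projectile that explodes on a timer to instantly kill nearby enemies.
; On projectile movement activation, it sets initial speed from GrannySmith's Power.
; A Delay on Tick triggers a multi-sphere trace every few seconds, calling InstantDeath on any ImpEnemy, HighImp or HellMouth found.
; The ball destroys itself and spawns the explosion emitter only when such an enemy is hit; an older single-trace damage check is unused.
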(event OnComponentActivated(ProjectileMovement)
  (params (Component :type Actor%20Component%20Object%20Reference) (bReset :type Boolean))
  (bind _asgranny_smith (Utilities|Casting|CastToGrannySmith (Game|GetPlayerCharacter 0)))
  (bind _output_get (Variables|Default|SetSpeed (Variables|/Game/2DSideScrollerBP/Characters/GrannySmith.GrannySmith_C|GetPower _asgranny_smith)))
  (Variables|/Script/Engine.ProjectileMovementComponent|SetInitialSpeed (Variables|Default|GetProjectileMovement) (* _output_get 13.0)))

(event OnProjectileStop(ProjectileMovement)
  (params (ImpactResult :type Hit%20Result%20Structure%20%28by%20ref%29)))

(event Custom|TriggerExplosion
  (bind _sphere (Variables|Default|GetSphere))
  (bind _returnvalue (Transformation|GetWorldLocation _sphere))
  (bind (_outhits _returnvalue_2) (Collision|MultiSphereTraceForObjects _returnvalue (+ _returnvalue "1.000000, 0, 0") 5e+02 (Variables|Default|GetObjectTypes) false 0 "None"))
  (if _returnvalue_2
    (for _array_element _outhits
      (if (== (.HitActor (Collision|BreakHitResult _array_element)) (.AsImp%20Enemy (Utilities|Casting|CastToImpEnemy (.HitActor (Collision|BreakHitResult _array_element)))))
        (bind _asimp_enemy (Utilities|Casting|CastToImpEnemy (.HitActor (Collision|BreakHitResult _array_element))))
        (Default|InstantDeath _asimp_enemy)
        (Actor|DestroyActor :!label _label)
        (Effects|SpawnEmitterAttached "/Game/StarterContent/Particles/P_Explosion.P_Explosion" (Variables|Default|GetSphere) "None" "0, 0, 0" "0, 0, 0" "2.000000,2.000000,2.000000")
        (elif (== (.HitActor (Collision|BreakHitResult _array_element)) (.AsHigh%20Imp (Utilities|Casting|CastToHighImp (.HitActor (Collision|BreakHitResult _array_element)))))
          (bind _ashigh_imp (Utilities|Casting|CastToHighImp (.HitActor (Collision|BreakHitResult _array_element))))
          (Default|InstantDeath _ashigh_imp)
          (goto _label)
          (elif (== (.HitActor (Collision|BreakHitResult _array_element)) (.AsHell%20Mouth (Utilities|Casting|CastToHellMouth (.HitActor (Collision|BreakHitResult _array_element)))))
            (bind _ashell_mouth (Utilities|Casting|CastToHellMouth (.HitActor (Collision|BreakHitResult _array_element))))
            (Default|InstantDeath _ashell_mouth)
            (goto _label)))))))

(event EventBeginPlay)

(event Collision|EventActorBeginOverlap
  (params (OtherActor :type Actor%20Object%20Reference)))

(event EventTick
  (params (DeltaSeconds :type Float%20%28single-precision%29))
  (Utilities|FlowControl|Delay 3.0)
  (Development|PrintString "BOOM" true true "(R=0.000000,G=0.660000,B=1.000000,A=1.000000)" 1.0)
  (CallFunction|TriggerExplosion))

(fn ConstructionScript)