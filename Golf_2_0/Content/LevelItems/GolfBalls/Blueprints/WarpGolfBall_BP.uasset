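; Golf ball projectile that marks a warp destination for the player, GrannySmith, where it comes to rest.
; On movement activation, launch speed is scaled from the player's Power.
; On stop, it plays a teleport sound, sets the player's warp flag and location (Y zeroed, raised by capsule half-height), then destroys itself after a short delay.
; Tick polls a hell-mouth flag to destroy consumed balls.
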(event OnComponentActivated(ProjectileMovement)
  (params (Component :type Actor%20Component%20Object%20Reference) (bReset :type Boolean))
  (bind _asgranny_smith (Utilities|Casting|CastToGrannySmith (Game|GetPlayerCharacter 0)))
  (bind _output_get (Variables|Default|SetSpeed (Variables|/Game/2DSideScrollerBP/Characters/GrannySmith.GrannySmith_C|GetPower _asgranny_smith)))
  (Variables|/Script/Engine.ProjectileMovementComponent|SetInitialSpeed (Variables|Default|GetProjectileMovement) (* _output_get 13.0)))

(event OnProjectileStop(ProjectileMovement)
  (params (ImpactResult :type Hit%20Result%20Structure%20%28by%20ref%29))
  (bind _sphere (Variables|Default|GetSphere))
  (bind _returnvalue (Transformation|GetWorldLocation _sphere))
  (bind _asgranny_smith (Utilities|Casting|CastToGrannySmith (Game|GetPlayerCharacter 0)))
  (Variables|/Game/2DSideScrollerBP/Characters/GrannySmith.GrannySmith_C|SetbIsWarping _asgranny_smith true)
  (Audio|PlaySound2D "/Game/Assets/Sounds/Ball_SFX/Warp_Ball_Teleport.Warp_Ball_Teleport" 1.0 1.0 0.0 0 0)
  (Variables|/Game/2DSideScrollerBP/Characters/GrannySmith.GrannySmith_C|SetWarpLocation _asgranny_smith (Math|Vector|MakeVector (.x _returnvalue) 0.0 (+ (/ (Components|Capsule|GetScaledCapsuleHalfHeight (Variables|/Script/Engine.Character|GetCapsuleComponent _asgranny_smith)) 1.0) (.z _returnvalue))))
  (Utilities|FlowControl|Delay 0.2)
  (Actor|DestroyActor))

(event Custom|consumedByHellMouth
  (Actor|DestroyActor))

(event EventBeginPlay)

(event Collision|EventActorBeginOverlap
  (params (OtherActor :type Actor%20Object%20Reference)))

(event EventTick
  (params (DeltaSeconds :type Float%20%28single-precision%29))
  (if (Variables|Default|GetbConsumedByHellMouth)
    (CallFunction|ConsumedbyHellMouth)))

(fn ConstructionScript)