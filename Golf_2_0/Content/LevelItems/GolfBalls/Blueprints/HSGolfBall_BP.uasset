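; HSGolfBall_BP is a golf ball projectile that homes on a PaperCharacter and takes its launch speed from the player.
; On BeginPlay it loops over all PaperCharacters, assigning each capsule as homing target, so the last one found wins.
; When ProjectileMovement activates, it sets InitialSpeed from the GrannySmith player's Power times a constant.
; The ball destroys itself when the projectile stops.
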(event OnComponentActivated(ProjectileMovement)
  (params (Component :type Actor%20Component%20Object%20Reference) (bReset :type Boolean))
  (bind _asgranny_smith (Utilities|Casting|CastToGrannySmith (Game|GetPlayerCharacter 0)))
  (bind _output_get (Variables|Default|SetSpeed (Variables|/Game/2DSideScrollerBP/Characters/GrannySmith.GrannySmith_C|GetPower _asgranny_smith)))
  (Variables|/Script/Engine.ProjectileMovementComponent|SetInitialSpeed (Variables|Default|GetProjectileMovement) (* _output_get 13.0)))

(event OnProjectileStop(ProjectileMovement)
  (params (ImpactResult :type Hit%20Result%20Structure%20%28by%20ref%29))
  (Actor|DestroyActor))

(event EventBeginPlay
  (bind _outactors (Actor|GetAllActorsOfClass "/Script/Paper2D.PaperCharacter"))
  (for _array_element _outactors
    (Variables|/Script/Engine.ProjectileMovementComponent|SetHomingTargetComponent (Variables|Default|GetProjectileMovement) (Variables|/Script/Engine.Character|GetCapsuleComponent _array_element))))

(event Collision|EventActorBeginOverlap
  (params (OtherActor :type Actor%20Object%20Reference)))

(event EventTick
  (params (DeltaSeconds :type Float%20%28single-precision%29)))

(fn ConstructionScript)